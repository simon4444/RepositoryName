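; MyGameManager is a game manager Blueprint that holds the current game state and switches UI and mouse cursor visibility to match it.
; Init creates the abandon widget, adds it to the viewport and sets the state to Running.
; SetState hides the UI, stores the new state, then hides the mouse for Running or shows the abandon widget and mouse for Abandon.
; GetState returns the current state, and the event graph is unused.
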(event EventBeginPlay)

(event Collision|EventActorBeginOverlap
  (params (OtherActor :type Actor%20Object%20Reference)))

(event EventTick
  (params (DeltaSeconds :type Float%20%28single-precision%29)))

(fn ConstructionScript)

(fn Init
  (CallFunction|CreateUI)
  (CallFunction|SetState "NewEnumerator0"))

(fn SetState
  (params (NewState :type MyGameStates%20Enum :default "NewEnumerator0"))
  (CallFunction|HideUI)
  (bind _output_get (Variables|Default|SetCurrentGameState NewState))
  (switch Utilities|FlowControl|Switch|SwitchonMyGameStates _output_get
    (:NewEnumerator0
      (CallFunction|ShowMouse false))
    (:NewEnumerator3
      (Widget|SetVisibility (Variables|Default|GetWidget_Abandon) "Visible")
      (CallFunction|ShowMouse true))))

(fn GetState
  (return (Variables|Default|GetCurrentGameState)))

(fn CreateUI
  (bind _returnvalue (UserInterface|CreateWidget "/Game/__MyContent/UI/Widget_abandon.Widget_abandon_C"))
  (bind _output_get (Variables|Default|SetWidget_Abandon _returnvalue))
  (UserInterface|Viewport|AddtoViewport _output_get 0))