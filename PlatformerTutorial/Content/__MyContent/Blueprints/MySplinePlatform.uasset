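; A moving platform actor whose mesh travels along a spline.
; On BeginPlay a timeline starts at a configurable play rate, and its SplineDistance track, scaled by the spline length, sets the mesh's world location on each update without sweeping.
; The construction script applies the configurable static mesh and material to the platform.
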(event Custom|PlatformStart
  (bind _spline (Variables|Default|GetSpline))
  (bind _spline_distance (Timeline|Motion%20Timeline PlayFromStart)
    (:Update
      (Transformation|SetWorldLocation (Variables|Default|GetPlatformMesh) (Spline|GetLocationatDistanceAlongSpline _spline (* _spline_distance (Spline|GetSplineLength _spline)) "World") false false))))

(event EventBeginPlay
  (bind _motion_timeline (Variables|Default|GetMotion%20Timeline))
  (CallFunction|PlatformStart)
  (Components|Timeline|SetPlayRate _motion_timeline (Variables|Default|GetRate))
  (Components|Timeline|PlayfromStart _motion_timeline))

(fn ConstructionScript
  (bind _platformmesh (Variables|Default|GetPlatformMesh))
  (Components|StaticMesh|SetStaticMesh _platformmesh (Variables|Default|GetStaticMesh))
  (Rendering|Material|SetMaterial _platformmesh 0 (Variables|Default|GetMaterial)))